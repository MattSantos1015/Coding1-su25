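; BP_Key is a collectible key pickup that the player gathers by walking into it.
; When BoxCollider overlaps an actor that casts to ThirdPersonCharacterCustom, it increments that character's KeyCount and destroys itself.
; Debug prints report spawn, pickup, the new key total and failed casts.
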(event `self.ReceiveBeginPlay`
  (`KismetSystemLibrary.PrintString` "This Key exists!" true true (struct :`R` 0.664006 :`G` 0.2468 :`B` 1.0 :`A` 1.0)))

(event `self.BoxCollider.OnComponentBeginOverlap`
  (params (OverlappedComponent :type "PrimitiveComponent Object Reference") (OtherActor :type "Actor Object Reference") (OtherComp :type "PrimitiveComponent Object Reference") (OtherBodyIndex :type Integer) (bFromSweep :type Boolean) (SweepResult :type "HitResult Structure (by ref)"))
  (bind _asthird_person_character_custom (cast `/Game/Blueprints/ThirdPersonCharacterCustom` OtherActor)
    (:`then`
      (`KismetSystemLibrary.PrintString` "Key has been overlapped by playr" true true (struct :`G` 0.66 :`B` 1.0 :`A` 1.0) 5.0)
      (bind _keycount (`/Game/Blueprints/ThirdPersonCharacterCustom.keyCount` _asthird_person_character_custom))
      (set `/Game/Blueprints/ThirdPersonCharacterCustom.keyCount` (+ _keycount 1) _asthird_person_character_custom) ; Set keyCount
      (`KismetSystemLibrary.PrintString` (`KismetStringLibrary.Concat_StrStr` "The Player has " (`KismetStringLibrary.Conv_IntToString` _keycount) " key(s)") true true (struct :`G` 0.66 :`B` 1.0 :`A` 1.0) 5.0)
      (`self.K2_DestroyActor`) ; DestroysThisKey
    )
    (:`CastFailed`
      (`KismetSystemLibrary.PrintString` "Key player cast failed!" true true (struct :`R` 1.0 :`B` 0.015071 :`A` 1.0) 5.0))))

(fn `UserConstructionScript`)