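; Tutorial-style test actor that demonstrates loops and arrays in Blueprint, mostly through on-screen debug prints.
; BeginPlay starts a delayed endless print loop, enables input and gathers all BP_Key actors.
; ChangeKeyColors re-calls itself after a delay, recoloring one key per pass through dynamic materials and reshuffling keys and colors on wrap.
; Tick logs frame counts, input triggers while-loop and name-array demos, and RecursiveLoop is defined but never started.
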(event `self.ReceiveBeginPlay`
  (`KismetSystemLibrary.PrintString` "Lists&Loops is running")
  (`|ExecutionSequence`
    (:`then_0`
      ; Setup for Loops
      (`self.Simple Game Loop`)
      (`self.EnableInput` (`GameplayStatics.GetPlayerController` 0)))
    (:`then_1`
      ;[0.15 0.1261 0.0601 0.5] Setup for Lists
      (bind _outactors (`GameplayStatics.GetAllActorsOfClass` "/Game/Blueprints/BP_Key.BP_Key_C"))
      (set `self.Keys` _outactors)
      (`self.Change Key Colors`))))

(event `Simple Game Loop`
  (`KismetSystemLibrary.PrintString` "Starting Game Loop" true true (struct :`G` 0.66 :`B` 1.0 :`A` 1.0) 0.6 :!label _label)
  (`KismetSystemLibrary.Delay` 1.0) ; Wait One Second
  (goto _label))

(event `self.ReceiveTick`
  (params (DeltaSeconds :type "Float (single-precision)"))
  (bind _result (`/Engine/EditorBlueprintResources/StandardMacros.IncrementInt` (`self.TickCounter`))
    (:`  `
      (`KismetSystemLibrary.PrintString` (`KismetStringLibrary.Concat_StrStr` "In even tick, We have run" (`KismetStringLibrary.Conv_IntToString` _result) "times") true true (struct :`R` 0.795356 :`G` 1.0 :`B` 0.087183 :`A` 1.0))
      (`KismetSystemLibrary.PrintString` (`KismetStringLibrary.Concat_StrStr` "The last frame took" (`KismetStringLibrary.Conv_DoubleToString` DeltaSeconds) "seconds to render") true true (struct :`R` 0.232021 :`B` 1.0 :`A` 1.0) 0.0))))

(event `InputAction|StartWhile loop`
  (params (Key :type "Key Structure"))
  (bind _while_loop_counter (`self.While loop counter`))
  (:`Pressed`
    (`KismetSystemLibrary.PrintString` "Starting WHile loop")
    (while (< (`self.While loop counter`) 25)
      ;[0.15 0.04611 0.1243 0.5] The while loops body
      (`/Engine/EditorBlueprintResources/StandardMacros.IncrementInt` _while_loop_counter
        (:`  `
          (`KismetSystemLibrary.PrintString` (`KismetStringLibrary.Concat_StrStr` "This while loop has run" (`KismetStringLibrary.Conv_IntToString` _while_loop_counter) " times") true true (`KismetMathLibrary.MakeColor` (`KismetMathLibrary.RandomFloat`) (`KismetMathLibrary.RandomFloat`) (`KismetMathLibrary.RandomFloat`))))))
    (`KismetSystemLibrary.PrintString` "The while loop is complete")
    (set `self.While loop counter` 0) ; Resests while loop counter to zero
  ))

(event `Recursive Loop`
  ;[0 0.111 0.15 0.5] Recursive Loop (Calls Itself)
  (if (< (`self.Recurion counter`) 5)
    (bind _result (`/Engine/EditorBlueprintResources/StandardMacros.IncrementInt` (`self.Recurion counter`))
      (:`  `
        (`KismetSystemLibrary.PrintString` (`KismetStringLibrary.Concat_StrStr` "The recursive loop has run" (`KismetStringLibrary.Conv_IntToString` _result) " times.") true true (`KismetMathLibrary.MakeColor` (`KismetMathLibrary.RandomFloat`) (`KismetMathLibrary.RandomFloat`) (`KismetMathLibrary.RandomFloat`)) 1.0)
        (`KismetSystemLibrary.Delay` 2.0)))
    (else
      (`KismetSystemLibrary.PrintString` "Resetting Recursive Loop")
      (set `self.Recurion counter` 0)
      (`KismetSystemLibrary.Delay` 5.0)))
  (`self.Recursive Loop`))

(event `Key|Six`
  (params (Key :type "Key Structure"))
  (:`Pressed`
    (`self.First Array Test`)))

(event `First Array Test`
  (bind _array (`|MakeArray` "Chewie" "Luke " "Leia" "Han" "Artoo" "Threepio"))
  (`KismetSystemLibrary.PrintString` (`KismetStringLibrary.Concat_StrStr` "our array of  names has " (`KismetStringLibrary.Conv_IntToString` (`KismetArrayLibrary.Array_Length` _array)) " int it"))
  (`KismetSystemLibrary.PrintString` (`KismetStringLibrary.Concat_StrStr` "The first name in the array is " (`|GetArrayItem` _array))))

(event `Key|Five`
  (params (Key :type "Key Structure"))
  (:`Pressed`
    (`self.List all names`)))

(event `List all names`
  (for (_array_element _array_index) (`|MakeArray` "Chewie" "Luke " "Leia" "Han" "Artoo" "Threepio")
    (`KismetSystemLibrary.PrintString` (`KismetStringLibrary.Concat_StrStr` (`KismetStringLibrary.Conv_IntToString` (+ _array_index 1)) "." _array_element))))

(event `Change Key Colors`
  (bind _keys (`self.Keys`))
  (bind _output (`|GetArrayItem` _keys (`self.Color Key Index`)))
  (if (or (>= (`self.Color Key Index`) (`KismetArrayLibrary.Array_Length` (`self.Colors`))) (>= (`self.Color Key Index`) (`KismetArrayLibrary.Array_Length` (`self.Keys`))))
    ;[0.15 0.03188 0.05197 0.5] Shuggle and reset
    (`KismetArrayLibrary.Array_Shuffle` (`self.Colors`)) ; Shuffles the order of colors
    (`KismetArrayLibrary.Array_Shuffle` _keys) ; Shuffles the order of keys
    (set `self.Color Key Index` 0))
  (`/Engine/EditorBlueprintResources/StandardMacros.IsValid` _output ; Checks if the keys exist
    (:`Is Valid`
      ;[0.1352 0.05962 0.15 0.5] Setting the Color
      (bind _returnvalue (`PrimitiveComponent.CreateDynamicMaterialInstance` (`/Game/Blueprints/BP_Key.Cylinder` _output) 0 "/Game/Materials/M_Base.M_Base" "None"))
      (`MaterialInstanceDynamic.SetVectorParameterValue` _returnvalue "Base Color" (`KismetMathLibrary.Conv_ColorToLinearColor` (`|GetArrayItem` (`self.Colors`) (`self.Color Key Index`)))))
    (:`Is Not Valid`
      ;[0.15 0.02347 0.01982 0.5] Resets the array of Keys if one is missing
      (bind _outactors (`GameplayStatics.GetAllActorsOfClass` "/Game/Blueprints/BP_Key.BP_Key_C"))
      (set `self.Keys` _outactors)))
  (`/Engine/EditorBlueprintResources/StandardMacros.IncrementInt` (`self.Color Key Index`)
    (:`  `
      (`KismetSystemLibrary.Delay` 0.5)
      (`self.Change Key Colors`))))

(fn `UserConstructionScript`)