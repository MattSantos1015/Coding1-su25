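; Wave manager that spawns one BP_Enemy at every BP_EnemySpanwer in the level and restarts the wave once the count runs out.
; BeginPlay caches the spawners, then each spawn takes the spawner's location and rotation, receives a reference to the manager and increments a live count.
; RemoveEnemyandCheck decrements that count and, at zero or below, announces a new wave and respawns after a short delay.
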(event `self.ReceiveBeginPlay`
  (`KismetSystemLibrary.PrintString` "Enemy Spawn Manager is Ready!")
  (bind _outactors (`GameplayStatics.GetAllActorsOfClass` "/Game/Blueprints/Enemies/BP_EnemySpanwer.BP_EnemySpanwer_C"))
  (set `self.Spawners` _outactors)
  (`self.Spawn Enemis`))

(event `Spawn Enemis`
  (for _array_element (`self.Spawners`)
    (bind (_returnvalue_location _returnvalue_rotation) (`KismetMathLibrary.BreakTransform` (`SceneComponent.K2_GetComponentToWorld` (`/Game/Blueprints/Enemies/BP_EnemySpanwer.DefaultSceneRoot` _array_element))))
    (bind _returnvalue (`|SpawnActorFromClass` "/Game/Blueprints/Enemies/BP_Enemy.BP_Enemy_C" (`KismetMathLibrary.MakeTransform` _returnvalue_location _returnvalue_rotation) "Undefined" "MultiplyWithRoot" null null)) ; Creates enemy as spawner locations + Rotation
    (set `/Game/Blueprints/Enemies/BP_Enemy.Manger` self _returnvalue) ; Assign this manager to the manager variable on each enemy.
    (`/Engine/EditorBlueprintResources/StandardMacros.IncrementInt` (`self.currentEnemiestotal`))))

(event `RemoveEnemyandCheck`
  (`/Engine/EditorBlueprintResources/StandardMacros.DecrementInt` (`self.currentEnemiestotal`)
    (:`  `
      (if (not (> (`self.currentEnemiestotal`) 0))
        (`KismetSystemLibrary.PrintString` "New Wave Incoming" true true (struct :`G` 0.66 :`B` 1.0 :`A` 1.0) 5.0)
        (`KismetSystemLibrary.Delay` 5.0)
        (`self.Spawn Enemis`)))))

(fn `UserConstructionScript`)